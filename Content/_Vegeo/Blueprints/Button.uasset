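; Button actor that switches a spotlight on while the first-person player character stands inside its Detector volume.
; On BeginPlay it caches the SpotLightComponent found by child index under Spotlight and sets its intensity to zero.
; Detector overlap begin raises the intensity and overlap end returns it to zero through the same turn-off path, each printing a debug message.
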(event `self.ReceiveBeginPlay`
  (bind _asspot_light_component (cast `SpotLightComponent` (`SceneComponent.GetChildComponent` (`SceneComponent.GetChildComponent` (`self.Spotlight`) 0) 1)))
  (set `self.As Spot Light Component` _asspot_light_component)
  (`LightComponent.SetIntensity` (`self.As Spot Light Component`) 0.0 :!label _label)
  (`KismetSystemLibrary.PrintString` "Turn Off"))

(event `self.Detector.OnComponentBeginOverlap`
  (params (OverlappedComponent :type "PrimitiveComponent Object Reference") (OtherActor :type "Actor Object Reference") (OtherComp :type "PrimitiveComponent Object Reference") (OtherBodyIndex :type Integer) (bFromSweep :type Boolean) (SweepResult :type "HitResult Structure (by ref)"))
  (cast `/Game/FirstPerson/Blueprints/BP_FirstPersonCharacter` OtherActor)
  (`LightComponent.SetIntensity` (`self.As Spot Light Component`) 800.0)
  (`KismetSystemLibrary.PrintString` "Turn On"))

(event `self.Detector.OnComponentEndOverlap`
  (params (OverlappedComponent :type "PrimitiveComponent Object Reference") (OtherActor :type "Actor Object Reference") (OtherComp :type "PrimitiveComponent Object Reference") (OtherBodyIndex :type Integer))
  (cast `/Game/FirstPerson/Blueprints/BP_FirstPersonCharacter` OtherActor)
  (goto _label))

(fn `UserConstructionScript`)