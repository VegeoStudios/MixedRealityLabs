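; MovingTarget is a Blueprint that moves its Target component back and forth between two marker components, Pos1 and Pos2.
; Each Tick sets Target's world location by lerping between the markers, using a sine of real time scaled by Speed and remapped to 0–1.
; The motion eases at each end and follows real time rather than game time, with no sweep for collision.
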(event `self.ReceiveTick`
  (params (DeltaSeconds :type "Float (single-precision)"))
  (`SceneComponent.K2_SetWorldLocation` (`self.Target`) (`KismetMathLibrary.VLerp` (`SceneComponent.K2_GetComponentLocation` (`self.Pos1`)) (`SceneComponent.K2_GetComponentLocation` (`self.Pos2`)) (* (+ (`KismetMathLibrary.Sin` (* (`GameplayStatics.GetRealTimeSeconds`) (`self.Speed`))) 1.0) 0.5)) false false))

(fn `UserConstructionScript`)