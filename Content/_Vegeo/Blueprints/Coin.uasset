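; Coin is a collectible pickup actor that adds to a score when the first-person player touches it.
; On begin play it finds the LabDebugObject in the level and uses it as the score store.
; Player overlap increments that Score, prints the new value and destroys the coin.
; Each tick the mesh bobs vertically on a sine of real time and spins at a fixed per-frame step.
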(event `self.ReceiveBeginPlay`
  (bind _returnvalue (`GameplayStatics.GetActorOfClass` "/Game/_Vegeo/Blueprints/LabDebugObject.LabDebugObject_C"))
  (set `self.ScoreStorer` _returnvalue))

(event `self.ReceiveActorBeginOverlap`
  (params (OtherActor :type "Actor Object Reference"))
  (cast `/Game/FirstPerson/Blueprints/BP_FirstPersonCharacter` OtherActor)
  (bind _result (`/Engine/EditorBlueprintResources/StandardMacros.IncrementInt` (`/Game/_Vegeo/Blueprints/LabDebugObject.Score` (`self.ScoreStorer`)))
    (:`  `
      (`KismetSystemLibrary.PrintString` (`KismetStringLibrary.Concat_StrStr` "Score is now: " (`KismetStringLibrary.Conv_IntToString` _result)))
      (`self.K2_DestroyActor`))))

(event `self.ReceiveTick`
  (params (DeltaSeconds :type "Float (single-precision)"))
  (bind _staticmesh (`self.StaticMesh`))
  (`SceneComponent.K2_SetRelativeLocation` _staticmesh (* (`KismetMathLibrary.Vector_Up`) (+ (* (`KismetMathLibrary.Sin` (`GameplayStatics.GetRealTimeSeconds`)) 20.0) 100.0)) false false)
  (`SceneComponent.K2_AddRelativeRotation` _staticmesh (struct :`Yaw` 1.0) false false))

(fn `UserConstructionScript`)